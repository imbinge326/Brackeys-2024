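; BP_Bullet is a bullet actor that applies a radial impulse and destroys itself when it hits something.
; On BeginPlay it spawns a particle effect at its own transform and plays a sound at the world origin rather than at the bullet.
; When the Collider component registers a hit, it fires the RadialForce impulse, spawns an impact particle and sound at the hit location, then destroys the actor.
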(event OnComponentHit(Collider)
  (params (HitComponent :type Primitive%20Component%20Object%20Reference) (OtherActor :type Actor%20Object%20Reference) (OtherComp :type Primitive%20Component%20Object%20Reference) (NormalImpulse :type Vector :default "0, 0, 0") (Hit :type Hit%20Result%20Structure%20%28by%20ref%29))
  (bind _location (Collision|BreakHitResult Hit))
  (Class|RadialForceComponent|FireImpulse (Variables|Default|GetRadialForce))
  (Effects|SpawnEmitteratLocation "/Engine/Functions/Engine_MaterialFunctions02/ExampleContent/3dParticleOpacity_Particle.3dParticleOpacity_Particle" _location)
  (Audio|PlaySoundatLocation "/Engine/EditorSounds/Notifications/CompileStart_Cue.CompileStart_Cue" _location "0, 0, 0" 1.0 1.0 0.0 0 0 0 0)
  (Actor|DestroyActor))

(event EventBeginPlay
  (Audio|PlaySoundatLocation "/Engine/EditorSounds/GamePreview/PossessPlayer_Cue.PossessPlayer_Cue" "0, 0, 0" "0, 0, 0" 1.0 1.0 0.0 0 0 0 0)
  (Effects|SpawnEmitteratLocation "/Engine/Tutorial/SubEditors/TutorialAssets/TutorialParticleSystem.TutorialParticleSystem" (Transformation|GetActorLocation) (Transformation|GetActorRotation)))

(event Collision|EventActorBeginOverlap
  (params (OtherActor :type Actor%20Object%20Reference)))

(event EventTick
  (params (DeltaSeconds :type Float%20%28single-precision%29)))

(fn ConstructionScript)